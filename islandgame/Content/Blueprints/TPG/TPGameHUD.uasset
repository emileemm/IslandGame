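; HUD for a timed pickup game that draws the countdown and score and also holds that game state.
; BeginPlay calls StartGame to reset score, time, key and game-over state, then start a looping one-second timer that flags game over at zero.
; Coin pickups add score and clock pickups add time.
; DrawTextToScreen opens or closes a gate in DrawHUD to show or hide prompt text, such as an interact hint.
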(event `self.ReceiveDrawHUD`
  (params (SizeX :type Integer) (SizeY :type Integer))
  ;[1 1 1] visual timer and score on screen
  (`|ExecutionSequence`
    (:`then_0`
      (`self.DrawText` (`KismetStringLibrary.Conv_IntToString` (`self.time`)) (struct :`A` 1) 10.0 10.0 null 3.0)
      (`self.DrawText` (`KismetStringLibrary.Conv_IntToString` (`self.score`)) (struct :`A` 1) 1050.0 10.0 null 3.0))
    (:`then_1`
      ;[1 1 1] display "press e to interact" text when in log trigger
      (`/Engine/EditorBlueprintResources/StandardMacros.Gate` true :!label _label
        (:`Exit`
          (`self.DrawText` (stale `DrawTextToScreen` Text) (struct :`A` 1) 500.0 100.0 null 3.0))))))

(event `DrawTextToScreen`
  (params (Draw :type Boolean) (Text :type String))
  ;[1 1 1] display "press e to interact" text when in log trigger
  (if Draw
    (goto _label :!via `Open`)
    (else
      (goto _label :!via `Close`))))

(event `timer`
  ;[1 0 0] timer - decrements time by 1 and checks for game over
  (bind _result (`/Engine/EditorBlueprintResources/StandardMacros.DecrementInt` (`self.time`))
    (:`  `
      (if (<= _result 0)
        (set `self.gameOver` true)
        (`KismetSystemLibrary.K2_ClearTimer` null "timer")))))

(event `self.ReceiveBeginPlay`
  (`self.startGame`))

(fn `clockCollected`
  (bind _time (`self.time`))
  (`/Engine/EditorBlueprintResources/StandardMacros.ManipulateIntInternal` _time (+ _time 5)))

(fn `coinCollected`
  (`/Engine/EditorBlueprintResources/StandardMacros.IncrementInt` (`self.score`)))

(fn `UserConstructionScript`)