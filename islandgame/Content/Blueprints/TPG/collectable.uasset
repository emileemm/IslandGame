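; Collectable coin actor that registers a pickup with the HUD and removes itself.
; Any actor overlap casts the first player controller's HUD to TPGameHUD, calls CoinCollected on it, then destroys the actor; a failed cast leaves it in place.
; The construction script applies the mesh and RotatingMovement rate, pivot and local-space settings from variables, so each instance can set its own look and spin.
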(event `self.ReceiveActorBeginOverlap`
  (params (OtherActor :type "Actor Object Reference"))
  (bind _astpgame_hud (cast `/Game/Blueprints/TPG/TPGameHUD` (`PlayerController.GetHUD` (`GameplayStatics.GetPlayerController` 0))))
  (bind _output_get (set `self.collectableGameHUD` _astpgame_hud))
  (`/Game/Blueprints/TPG/TPGameHUD.coinCollected` _output_get)
  (`self.K2_DestroyActor`))

(fn `UserConstructionScript`
  (bind _rotatingmovement (`self.RotatingMovement`))
  (`StaticMeshComponent.SetStaticMesh` (`self.StaticMesh`) (`self.Mesh`))
  (set `RotatingMovementComponent.RotationRate` (`self.Rotation Rate`) _rotatingmovement)
  (set `RotatingMovementComponent.PivotTranslation` (`self.PivotTranslation`) _rotatingmovement)
  (set `RotatingMovementComponent.bRotationInLocalSpace` (`self.RotationLocal`) _rotatingmovement))